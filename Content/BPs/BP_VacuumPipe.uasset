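; Vacuum pipe actor that pulls overlapping components to its PlayerCenter point and holds them until VacuumDisable is triggered.
; A MoveComponentTo re-fires while the Keypress flag stays true; disabling shows a crossed hologram, then restores the vacuum material after a delay.
; Hover briefly shows the hologram mesh, hiding it by timer.
; A looping timer optionally oscillates another pipe mesh along X with a sine wave.
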(event OnComponentBeginOverlap(ActorCol)
  (params (OverlappedComponent :type Primitive%20Component%20Object%20Reference) (OtherActor :type Actor%20Object%20Reference) (OtherComp :type Primitive%20Component%20Object%20Reference) (OtherBodyIndex :type Integer) (bFromSweep :type Boolean) (SweepResult :type Hit%20Result%20Structure%20%28by%20ref%29))
  ;[1 1 1] Vacuum Pipe Functionality
  (Variables|Default|SetKeypress true)
  (Variables|Default|SetHasActor true)
  (Components|MoveComponentTo OtherComp (Transformation|GetWorldLocation (Variables|Default|GetPlayerCenter)) "0, 0, 0" false false 0.1 false :!label _label)
  (if (Variables|Default|GetKeypress)
    (Utilities|FlowControl|ForLoopwithBreak 0 0
      (:LoopBody
        (goto _label)))
    (else
      (Variables|Default|SetHasActor false)
      (Utilities|FlowControl|Delay 3.0) ; This is to stop the vacuum from immediately picking up actors after the keypress
      (Rendering|Material|CreateDynamicMaterialInstance (Variables|Default|GetSM_Pipe_Straight_Short) 0 "/Game/Materials/BPs/Vacuum/M_MasterHologram_Vacuum_Inst.M_MasterHologram_Vacuum_Inst" "None" :!class /Script/Engine.PrimitiveComponent)
      (goto _label Stop))))

(event Custom|Back&ForthCheck
  ;[1 1 1] Back and Forth Movement
  (if (Variables|Default|GetBack_Forth)
    (Transformation|SetRelativeLocation (Variables|Default|GetSM_Pipe_Straight_Short_03) (Math|Vector|MakeVector (* (Math|Trig|Sin(Radians) (* (Utilities|Time|GetGameTimeinSeconds) (Variables|Default|GetFreq))) (Variables|Default|GetAmp)) 0.0 0.0) false false)))

(event Custom|NoLongerHoveringEvent
  ;[1 1 1] Hologram Visibility
  (Rendering|SetVisibility (Variables|Default|GetSM_Pipe_Straight_Short) false false))

(event EventBeginPlay
  ;[1 1 1] Enables Input
  (Input|EnableInput (Game|GetPlayerController 0))
  ;[1 1 1] Back and Forth Movement
  (Utilities|Time|SetTimerbyEvent (delegate Custom|Back&ForthCheck) 0.01 true))

(event EventVacuumDisable
  ;[1 1 1] Vacuum Pipe Functionality
  (Variables|Default|SetKeypress false)
  (if (Variables|Default|GetHasActor)
    (Rendering|Material|CreateDynamicMaterialInstance (Variables|Default|GetSM_Pipe_Straight_Short) 0 "/Game/Materials/BPs/Vacuum/M_MasterHologram_VacuumCross_Inst.M_MasterHologram_VacuumCross_Inst" "None" :!class /Script/Engine.PrimitiveComponent)))

(event EventHover
  ;[1 1 1] Hologram Visibility
  (Utilities|Time|SetTimerbyEvent (delegate Custom|NoLongerHoveringEvent) 0.01)
  (Rendering|SetVisibility (Variables|Default|GetSM_Pipe_Straight_Short) true false))

(fn ConstructionScript)