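; BP_TextPopUp is a trigger actor that shows a text prompt when an actor tagged Player enters its Box.
; On BeginPlay it writes NewPromptText into the PromptText of its W_InteractPrompt widget.
; Box overlaps toggle the widget component's visibility and the InsideBox flag, which nothing in this file reads.
; End overlap skips the tag check, so any actor leaving hides the prompt.
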(event OnComponentBeginOverlap(Box)
  (params (OverlappedComponent :type Primitive%20Component%20Object%20Reference) (OtherActor :type Actor%20Object%20Reference) (OtherComp :type Primitive%20Component%20Object%20Reference) (OtherBodyIndex :type Integer) (bFromSweep :type Boolean) (SweepResult :type Hit%20Result%20Structure%20%28by%20ref%29))
  ;[1 1 1] Show Widget when Player enters
  (if (Actor|ActorHasTag OtherActor "Player")
    (Rendering|SetVisibility (Variables|Default|GetWidget) true false)
    (Variables|Default|SetInsideBox true)))

(event OnComponentEndOverlap(Box)
  (params (OverlappedComponent :type Primitive%20Component%20Object%20Reference) (OtherActor :type Actor%20Object%20Reference) (OtherComp :type Primitive%20Component%20Object%20Reference) (OtherBodyIndex :type Integer))
  ;[1 1 1] Show Widget when Player enters
  (Rendering|SetVisibility (Variables|Default|GetWidget) false false)
  (Variables|Default|SetInsideBox false))

(event EventBeginPlay
  (bind _asw_interact_prompt (Utilities|Casting|CastToW_InteractPrompt (UserInterface|GetWidget (Variables|Default|GetWidget))))
  (Variables|/Script/UMG.TextBlock|SetText (Variables|/Game/BPs/Widgets/W_InteractPrompt.W_InteractPrompt_C|GetPrompt_Text _asw_interact_prompt) (Utilities|Text|ToText(String) (Variables|Default|GetNew%20Prompt%20Text))))

(fn ConstructionScript)