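; BP_Cube_02 is an actor whose cube component can oscillate back and forth along its relative Y axis.
; BeginPlay starts a fast looping timer that runs the check event.
; While the BackForth flag is set, that event sets the cube's Y location from a sine of game time scaled by Freq and Amp, using a timer instead of Tick.
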(event Custom|Back&ForthCheck
  (if (Variables|Default|GetBack_Forth)
    (Transformation|SetRelativeLocation (Variables|Default|GetCube) (Math|Vector|MakeVector 0.0 (* (Math|Trig|Sin(Radians) (* (Utilities|Time|GetGameTimeinSeconds) (Variables|Default|GetFreq))) (Variables|Default|GetAmp)) 0.0) false false)))

(event EventBeginPlay
  (Utilities|Time|SetTimerbyEvent (delegate Custom|Back&ForthCheck) 0.01 true))

(fn ConstructionScript)