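; BP_LauncherPipe is a pipe actor that launches characters and BP_Cube objects that overlap its colliders.
; Nested switches on truncated actor pitch and yaw select preset directional velocities for LaunchCharacter, overriding existing velocity.
; Cubes get a velocity-change impulse instead, with only the south slope and west slope velocities handled.
; A Hover event shows the straight pipe mesh as a hologram, and a very short timer hides it again.
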(event OnComponentBeginOverlap(PlayerCol)
  (params (OverlappedComponent :type Primitive%20Component%20Object%20Reference) (OtherActor :type Actor%20Object%20Reference) (OtherComp :type Primitive%20Component%20Object%20Reference) (OtherBodyIndex :type Integer) (bFromSweep :type Boolean) (SweepResult :type Hit%20Result%20Structure%20%28by%20ref%29))
  (bind _returnvalue (Transformation|GetActorRotation))
  (bind _returnvalue_2 (Math|Float|Truncate (.pitch _returnvalue)))
  ;[1 1 1] Character Launch Velocity based on this actor's Y and Z rotation
  (bind _ascharacter (Utilities|Casting|CastToCharacter OtherActor))
  (switch int _returnvalue_2
    (:Default
      (switch int _returnvalue_2
        (:Default
          (switch int _returnvalue_2
            (:Default
              (switch int _returnvalue_2
                (:Default
                  (switch int (Math|Float|Truncate (.yaw _returnvalue))
                    (:-90
                      (Character|LaunchCharacter _ascharacter (Variables|Velocities|GetWest%20Facing%20Slope%20Velocity) true true)
                      (if (Utilities|Operators|EqualEqual (Transformation|GetActorRotation) (Math|Rotator|MakeRotator 1.8e+02 0.0 1.8e+02) 0.1)
                        (Character|LaunchCharacter _ascharacter (Variables|Velocities|GetDown%20Facing%20Velocity) true true)))))
                (:90
                  (Character|LaunchCharacter _ascharacter (Variables|Velocities|GetNorth%20Facing%20Velocity) true true))))
            (:0
              (Character|LaunchCharacter _ascharacter (Variables|Velocities|GetUp%20Facing%20Velocity) true true))))
        (:35
          (Character|LaunchCharacter _ascharacter (Variables|Velocities|GetNorth%20Facing%20Slope%20Velocity) true true))))
    (:-35
      (Character|LaunchCharacter _ascharacter (Variables|Velocities|GetSouth%20Facing%20Slope%20Velocity%20) true true))))

(event OnComponentBeginOverlap(ObjectCol)
  (params (OverlappedComponent :type Primitive%20Component%20Object%20Reference) (OtherActor :type Actor%20Object%20Reference) (OtherComp :type Primitive%20Component%20Object%20Reference) (OtherBodyIndex :type Integer) (bFromSweep :type Boolean) (SweepResult :type Hit%20Result%20Structure%20%28by%20ref%29))
  (bind _returnvalue (Transformation|GetActorRotation))
  ;[1 1 1] Object Launch Velocity based on this actor's Y and Z rotation
  (bind _asbp_cube (Utilities|Casting|CastToBP_Cube OtherActor))
  (switch int (Math|Float|Truncate (.pitch _returnvalue))
    (:Default
      (switch int (Math|Float|Truncate (.yaw _returnvalue))
        (:-90
          (Physics|AddImpulse (Variables|/Game/BPs/BP_Cube.BP_Cube_C|GetCol _asbp_cube) (Variables|Velocities|GetWest%20Facing%20Slope%20Velocity) "None" true))))
    (:-35
      (Physics|AddImpulse (Variables|/Game/BPs/BP_Cube.BP_Cube_C|GetCol _asbp_cube) (Variables|Velocities|GetSouth%20Facing%20Slope%20Velocity%20) "None" true))))

(event Custom|NoLongerHoveringEvent
  ;[1 1 1] Hologram Visibility
  (Rendering|SetVisibility (Variables|Default|GetSM_Pipe_Straight_Short) false false))

(event EventHover
  ;[1 1 1] Hologram Visibility
  (Utilities|Time|SetTimerbyEvent (delegate Custom|NoLongerHoveringEvent) 0.01)
  (Rendering|SetVisibility (Variables|Default|GetSM_Pipe_Straight_Short) true false))

(fn ConstructionScript)