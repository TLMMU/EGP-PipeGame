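; BP_Button is an interactive button that spawns a BP_Cube when the player triggers IA_Button while inside its overlap box.
; A press plays the ButtonPress timeline, which pushes the button mesh down and blends the color of PowerLine-tagged meshes through dynamic material instances.
; In parallel, a short delay precedes spawning the cube at the SpawnTransform.
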(event OnComponentBeginOverlap(Box)
  (params (OverlappedComponent :type Primitive%20Component%20Object%20Reference) (OtherActor :type Actor%20Object%20Reference) (OtherComp :type Primitive%20Component%20Object%20Reference) (OtherBodyIndex :type Integer) (bFromSweep :type Boolean) (SweepResult :type Hit%20Result%20Structure%20%28by%20ref%29))
  (Variables|Default|SetInsideBox true))

(event OnComponentEndOverlap(Box)
  (params (OverlappedComponent :type Primitive%20Component%20Object%20Reference) (OtherActor :type Actor%20Object%20Reference) (OtherComp :type Primitive%20Component%20Object%20Reference) (OtherBodyIndex :type Integer))
  (Variables|Default|SetInsideBox false))

(event Input|EnhancedActionEvents|EnhancedInputActionIA_Button
  (params (ActionValue :type Boolean) (ElapsedSeconds :type Float%20%28double-precision%29) (TriggeredSeconds :type Float%20%28double-precision%29) (InputAction :type Input%20Action%20Object%20Reference :default "/Game/Input/IA_Button.IA_Button"))
  (if (Variables|Default|GetInsideBox)
    (Utilities|FlowControl|Sequence
      (:then_0
        (bind (_direction _press _light) (Timeline|ButtonPress PlayFromStart)
          (:Update
            (Transformation|SetRelativeLocation (Variables|Default|GetSM_Button) (Math|Vector|MakeVector 0.0 0.0 (Math|Float|Lerp 69.0 61.0 _press)) false false)
            (for _array_element (Actor|GetComponentsbyTag "/Script/Engine.StaticMeshComponent" "PowerLine")
              (bind _returnvalue (Rendering|Material|CreateDynamicMaterialInstance _array_element 0 "/Game/Materials/BPs/Button/M_PowerLine.M_PowerLine" "None" :!class /Script/Engine.PrimitiveComponent))
              (Rendering|Material|SetVectorParameterValue _returnvalue "Color" (Math|Color|Lerp(LinearColor) (Utilities|Struct|MakeLinearColor 1.0 1.0 1.0 0.0) (Utilities|Struct|MakeLinearColor 0.0 0.5 0.8 0.0) _light) :!class /Script/Engine.MaterialInstanceDynamic)))))
      (:then_1
        (Utilities|FlowControl|Delay 1.0)
        (Game|SpawnActorfromClass "/Game/BPs/BP_Cube.BP_Cube_C" (Variables|Default|GetSpawn%20Transform) "Undefined" "MultiplyWithRoot" 0 0)))))

(event EventBeginPlay
  (Input|EnableInput (Game|GetPlayerController 0)))

(fn ConstructionScript)